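; BP_Enemy1 is a ghost enemy with an invisible mesh until killed and a minimap sprite shown only on authority.
; A player entering its sphere starts a looping timer that turns it to face them until they leave.
; An interface kill event flattens the capsule, reveals the mesh through the IsHit RepNotify and notifies the spawner.
; After a delay it destroys itself and increments the GameState ghost-kill count.
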(event OnComponentBeginOverlap(Sphere)
  (params (OverlappedComponent :type Primitive%20Component%20Object%20Reference) (OtherActor :type Actor%20Object%20Reference) (OtherComp :type Primitive%20Component%20Object%20Reference) (OtherBodyIndex :type Integer) (bFromSweep :type Boolean) (SweepResult :type Hit%20Result%20Structure%20%28by%20ref%29))
  ;[1 1 1] OnTrigger face player
  (if (Actor|ActorHasTag OtherActor "Player")
    (Variables|Default|SetNearest%20Player OtherActor)
    (bind _returnvalue (Utilities|Time|SetTimerbyEvent (delegate Custom|Look%20At%20Player) 0.1 true))))

(event OnComponentEndOverlap(Sphere)
  (params (OverlappedComponent :type Primitive%20Component%20Object%20Reference) (OtherActor :type Actor%20Object%20Reference) (OtherComp :type Primitive%20Component%20Object%20Reference) (OtherBodyIndex :type Integer))
  ;[1 1 1] OnExit reset value
  (if (Actor|ActorHasTag OtherActor "Player")
    (Variables|Default|SetNearest%20Player 0)
    (Variables|Default|SetMinDistanceFound 99999.0)
    (Transformation|SetActorRotation self (Variables|Default|GetSelfRotation))
    (Utilities|Time|ClearandInvalidateTimerbyHandle (stale OnComponentBeginOverlap(Sphere) _returnvalue))))

(event Custom|Look%20At%20Player
  (bind _returnvalue (Transformation|GetActorLocation))
  (bind _nearest_player (Variables|Default|GetNearest%20Player))
  (bind _returnvalue_2 (Transformation|GetActorLocation _nearest_player))
  (bind _returnvalue_3 (Math|Rotator|FindLookatRotation _returnvalue _returnvalue_2))
  ;[1 1 1] OnTrigger face player
  (if (< (Math|Vector|Distance(Vector) _returnvalue _returnvalue_2) (Variables|Default|GetMinDistanceFound))
    (Variables|Default|SetMinDistanceFound (Variables|Default|GetMinDistanceFound))
    (Transformation|SetActorRotation _returnvalue_3)
    (Variables|Default|SetSelfRotation _returnvalue_3)))

(event Custom|ShowAndDestroyManny
  (bind _returnvalue (Game|GetGameState))
  (Utilities|Time|ClearandInvalidateTimerbyHandle (stale OnComponentBeginOverlap(Sphere) _returnvalue))
  (Components|Capsule|SetCapsuleHalfHeight (Variables|Collision|GetCapsuleComponent) 0.0 true)
  (Variables|Default|SetisKilled true)
  (Variables|Default|SetisHit true)
  (if (Utilities|IsValid self)
    (Class|BPIEnemySpawn|ESIEnemyKill(Message) (Variables|Default|GetSpawnerRef))
    (Utilities|FlowControl|Delay 5.0)
    (Actor|DestroyActor)
    (bind _ghostkill (Class|BPIGraveGameState|GGSIGetGhostKill(Message) _returnvalue))
    (bind _result (Math|Integer|IncrementInt _ghostkill)
      (:%20%20
        (Class|BPIGraveGameState|GGSISetGhostKill(Message) _returnvalue _result)))))

(event EventEISpawnandDestroyEnemy
  (if (not (Variables|Default|GetisKilled))
    (CallFunction|ShowandDestroyManny)))

(event EventBeginPlay
  ;[1 1 1] Disable Minimap Indication for client
  (Rendering|SetVisibility (Variables|Character|GetMesh) false false)
  (if (Ability|HasAuthority)
    (Rendering|SetVisibility (Variables|Default|GetPaperSprite) true false)
    (bind _returnvalue (Actor|GetActorOfClass "/Game/Blueprints/BP_EnemySpawner.BP_EnemySpawner_C"))
    (Variables|Default|SetSpawnerRef _returnvalue)))

(fn ConstructionScript)

(fn OnRepIsHit
  (Rendering|SetVisibility (Variables|Character|GetMesh) true false))