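; Game mode that assigns asymmetric Digger and Attacker roles to players as they log in.
; PostLogin switches on player controller count: the first player possesses a spawned Digger character, the second an Attacker spawned at an offset from that player's controller transform.
; Each branch records the role in BP_GravePlayerState.
; The first login also spawns an enemy spawner at the world origin after a short delay.
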(event EventPostLogin
  (params (NewPlayer :type Player%20Controller%20Object%20Reference))
  (switch int (Class|GameplayStatics|GetNumPlayerControllers)
    (:1
      (bind _returnvalue (Game|SpawnActorfromClass "/Game/Characters/BP_DiggerCharacter.BP_DiggerCharacter_C" (Transformation|GetActorTransform NewPlayer) "AdjustIfPossibleButAlwaysSpawn" "MultiplyWithRoot" 0 0))
      (Pawn|Possess NewPlayer _returnvalue)
      (bind _asbp_grave_player_state (Utilities|Casting|CastToBP_GravePlayerState (Variables|/Script/Engine.Controller|GetPlayerState NewPlayer)))
      (Variables|/Game/Blueprints/BP_GravePlayerState.BP_GravePlayerState_C|SetEStatePlayerRole _asbp_grave_player_state "NewEnumerator0")
      (Utilities|FlowControl|Delay 2.0)
      (Game|SpawnActorfromClass "/Game/Blueprints/BP_EnemySpawner.BP_EnemySpawner_C" (Math|Transform|MakeTransform "0, 0, 0") "AlwaysSpawn" "MultiplyWithRoot" 0 0))
    (:2
      (bind _returnvalue_2 (Game|SpawnActorfromClass "/Game/Characters/BP_AttackerCharacter.BP_AttackerCharacter_C" (Math|Transform|MakeTransform (+ (.location (Transformation|GetActorTransform NewPlayer)) "200.000000,0.000000,0.000000") "0.000000,270.000000,0.000000") "AdjustIfPossibleButAlwaysSpawn" "MultiplyWithRoot" 0 0))
      (Pawn|Possess NewPlayer _returnvalue_2)
      (bind _asbp_grave_player_state_2 (Utilities|Casting|CastToBP_GravePlayerState (Variables|/Script/Engine.Controller|GetPlayerState NewPlayer)))
      (Variables|/Game/Blueprints/BP_GravePlayerState.BP_GravePlayerState_C|SetEStatePlayerRole _asbp_grave_player_state_2 "NewEnumerator1"))))

(fn ConstructionScript)

(fn OnRepPRole)