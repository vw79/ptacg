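; BP_Extraction is an extraction zone that triggers the win screen once two players stand inside it.
; Box overlap events keep a running count of actors tagged Player, raised on entry and lowered on exit.
; Reaching two starts a short delay, then pushes the AWB_Win menu to the first player controller and pauses the game.
; The count is not rechecked after the delay, so leaving does not cancel the win.
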(event OnComponentBeginOverlap(Box)
  (params (OverlappedComponent :type Primitive%20Component%20Object%20Reference) (OtherActor :type Actor%20Object%20Reference) (OtherComp :type Primitive%20Component%20Object%20Reference) (OtherBodyIndex :type Integer) (bFromSweep :type Boolean) (SweepResult :type Hit%20Result%20Structure%20%28by%20ref%29))
  (bind _count (Variables|Default|GetCount))
  (if (Actor|ActorHasTag OtherActor "Player")
    (Math|Integer|IncrementInt _count
      (:%20%20
        (if (== _count 2)
          (Utilities|FlowControl|Delay 3.0)
          (Class|BPIPCWidgetManager|PCWMPushMenu(Message) (Game|GetPlayerController 0) "/Game/Widgets/AWB/AWB_Win.AWB_Win_C")
          (Game|SetGamePaused true))))))

(event OnComponentEndOverlap(Box)
  (params (OverlappedComponent :type Primitive%20Component%20Object%20Reference) (OtherActor :type Actor%20Object%20Reference) (OtherComp :type Primitive%20Component%20Object%20Reference) (OtherBodyIndex :type Integer))
  (if (Actor|ActorHasTag OtherActor "Player")
    (Math|Integer|DecrementInt (Variables|Default|GetCount))))

(fn ConstructionScript)