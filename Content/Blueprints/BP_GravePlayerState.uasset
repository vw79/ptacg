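; BP_GravePlayerState is a player state Blueprint that stores each player's nickname and Digger or Attacker role.
; PSI-prefixed functions and an event act as getters and setters for both values.
; A RepNotify on the role prints which role is being played, while the OnRep for StatePlayerName is empty and the name accessors use PlayerNickname instead.
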(event EventPSISetPlayerName
  (params (PlayerName :type Text))
  (Variables|Default|SetPlayerNickname PlayerName))

(fn ConstructionScript)

(fn OnRepEStatePlayerRole
  (switch Utilities|FlowControl|Switch|SwitchonPlayerRole (Variables|Default|GetEStatePlayerRole)
    (:NewEnumerator0
      (Development|PrintString "Playing as Digger"))
    (:NewEnumerator1
      (Development|PrintString "Playing as Attacker"))))

(fn OnRepStatePlayerName)

(fn PSIGetPlayerName
  (return (Variables|Default|GetPlayerNickname)))

(fn PSIGetPlayerRole
  (return (Variables|Default|GetEStatePlayerRole)))

(fn PSISetPlayerRole
  (params (PlayerRole :type PlayerRole%20Enum :default "NewEnumerator2"))
  (Variables|Default|SetEStatePlayerRole PlayerRole)
  (return))