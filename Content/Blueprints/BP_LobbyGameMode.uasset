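; Lobby game mode that sets up the two player roles, digger and attacker, as players join.
; PostLogin tracks controllers, spawns the matching menu pawn by join count (attacker offset and rotated from the start), possesses it and sets the role on BP_GravePlayerState.
; Logout removes the controller from the list.
; LGMShutdownLobby makes clients leave the EIK session first, then the first player, presumably the host, after a short delay.
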(event EventOnLogout
  (params (ExitingController :type Controller%20Object%20Reference))
  (bind _asplayer_controller (Utilities|Casting|CastToPlayerController ExitingController))
  (Utilities|Array|RemoveItem (Variables|Default|GetAllConnectedPlayer) _asplayer_controller))

(event EventLGMShutdownLobby
  (bind _allconnectedplayer (Variables|Default|GetAllConnectedPlayer))
  (for (_array_element _array_index) _allconnectedplayer
    (if (not (== _array_index 0))
      (Class|BPIPlayerController|PCILeaveEIKSession(Message) _array_element)))
  (Utilities|FlowControl|Delay 0.2)
  (Class|BPIPlayerController|PCILeaveEIKSession(Message) (Utilities|Array|Get(acopy) _allconnectedplayer)))

(event EventPostLogin
  (params (NewPlayer :type Player%20Controller%20Object%20Reference))
  (Utilities|Array|Add (Variables|Default|GetAllConnectedPlayer) NewPlayer)
  (switch int (Class|GameplayStatics|GetNumPlayerControllers)
    (:1
      (bind _returnvalue (Game|SpawnActorfromClass "/Game/Characters/BP_DiggerMenu.BP_DiggerMenu_C" (Transformation|GetActorTransform NewPlayer) "AdjustIfPossibleButAlwaysSpawn" "MultiplyWithRoot" 0 0))
      (Pawn|Possess NewPlayer _returnvalue)
      (bind _asbp_grave_player_state (Utilities|Casting|CastToBP_GravePlayerState (Variables|/Script/Engine.Controller|GetPlayerState NewPlayer)))
      (Variables|/Game/Blueprints/BP_GravePlayerState.BP_GravePlayerState_C|SetEStatePlayerRole _asbp_grave_player_state "NewEnumerator0"))
    (:2
      (bind _returnvalue_2 (Game|SpawnActorfromClass "/Game/Characters/BP_AttackerMenu.BP_AttackerMenu_C" (Math|Transform|MakeTransform (+ (.location (Transformation|GetActorTransform NewPlayer)) "0.000000,180.000000,0.000000") "0.000000,190.000000,0.000000") "AdjustIfPossibleButAlwaysSpawn" "MultiplyWithRoot" 0 0))
      (Pawn|Possess NewPlayer _returnvalue_2)
      (bind _asbp_grave_player_state_2 (Utilities|Casting|CastToBP_GravePlayerState (Variables|/Script/Engine.Controller|GetPlayerState NewPlayer)))
      (Variables|/Game/Blueprints/BP_GravePlayerState.BP_GravePlayerState_C|SetEStatePlayerRole _asbp_grave_player_state_2 "NewEnumerator1"))))

(fn ConstructionScript)