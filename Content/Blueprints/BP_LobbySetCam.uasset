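; BP_LobbySetCam switches the player view to a cine camera, apparently for the lobby.
; ServerSetClientCam checks authority on player controller 0, then calls MulticastSetCam.
; MulticastSetCam takes the CineCameraActor returned by GetActorOfClass and makes it the view target of player controller 0, with no blend time set.
; An unconnected copy of that camera logic with a debug print never runs.
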(event Custom|MulticastSetCam
  (bind _returnvalue (Actor|GetActorOfClass "/Script/CinematicCamera.CineCameraActor"))
  (Game|Player|SetViewTargetwithBlend (Game|GetPlayerController 0) _returnvalue 0.0 "VTBlend_Linear" 0.0 false))

(event Custom|ServerSetClientCam
  (if (Ability|HasAuthority (Game|GetPlayerController 0))
    (CallFunction|MulticastSetCam)))

(fn ConstructionScript)