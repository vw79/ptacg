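; Trigger box actor that shows the player dig UI when something overlaps its Box component.
; On begin overlap it checks that player 0's BP_GravePlayerState has the first role enum value, then uses a dot product to confirm the box lies in front of that player controller.
; If both pass, it creates and displays WBP_PlayerDig; end overlap removes the stored widget without any checks.
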(event OnComponentEndOverlap(Box)
  (params (OverlappedComponent :type Primitive%20Component%20Object%20Reference) (OtherActor :type Actor%20Object%20Reference) (OtherComp :type Primitive%20Component%20Object%20Reference) (OtherBodyIndex :type Integer))
  (Widget|RemovefromParent (Variables|Default|GetPlayerDigMenu)))

(event OnComponentBeginOverlap(Box)
  (params (OverlappedComponent :type Primitive%20Component%20Object%20Reference) (OtherActor :type Actor%20Object%20Reference) (OtherComp :type Primitive%20Component%20Object%20Reference) (OtherBodyIndex :type Integer) (bFromSweep :type Boolean) (SweepResult :type Hit%20Result%20Structure%20%28by%20ref%29))
  (bind _returnvalue (Game|GetPlayerController 0))
  (bind _asbp_grave_player_state (Utilities|Casting|CastToBP_GravePlayerState (Variables|/Script/Engine.Controller|GetPlayerState _returnvalue)))
  (if (Utilities|Enum|Equal(Enum) (Variables|/Game/Blueprints/BP_GravePlayerState.BP_GravePlayerState_C|GetEStatePlayerRole _asbp_grave_player_state) "NewEnumerator0")
    (bind _output_get (Variables|Default|SetDirectionToCollider (- (Transformation|GetActorLocation) (Transformation|GetActorLocation _returnvalue))))
    (if (> (Math|Vector|DotProduct (Transformation|GetActorForwardVector _returnvalue) _output_get) 0.0)
      (bind _returnvalue_2 (UserInterface|CreateWidget "/Game/Widgets/WBP_PlayerDig.WBP_PlayerDig_C"))
      (bind _output_get_2 (Variables|Default|SetPlayerDigMenu _returnvalue_2))
      (UserInterface|Viewport|AddtoViewport _output_get_2 0))))

(fn ConstructionScript)