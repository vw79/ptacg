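; Menu player controller that creates the base UI layout and pushes the play/login, lobby-create or lobby menu according to level name.
; Interface-style events push menus, HUD and prompts, while MasterBinderUI prompt results bound in Main Menu route to the active stack widget.
; In the lobby it fades in, blends to a cine camera and sends the nickname, with game-instance fallback, to PlayerState via server event.
; Leaving destroys EIK sessions and opens LobbyCreate.
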(event Custom|Bindings
  (bind _masterbinderui (Variables|Default|GetMasterBinderUI))
  ;[1 1 1] Exit Menu (Yes/ No)
  (EventDispatchers|AssignOnPromptConfirmed _masterbinderui (delegate Custom|OnPromptConfirmed_Event))
  (EventDispatchers|AssignOnPromptCanceled _masterbinderui (delegate Custom|OnPromptCanceled_Event)))

(event Custom|OnPromptConfirmed_Event
  (params (PromptIndex :type UI_PromptIndex%20Enum :default "NewEnumerator0") (PromptToStack :type UI_PromptToStack%20Enum :default "NewEnumerator0"))
  ;[1 1 1] Exit Menu (Yes/ No)
  (switch Utilities|FlowControl|Switch|SwitchonUI_PromptToStack PromptToStack
    (:NewEnumerator0
      (Class|BPIPromptInterface|PromptConfirmed(Message) (Class|CommonActivatableWidgetContainerBase|GetActiveWidget (Variables|/Game/Widgets/AWB/AWB_BaseUILayout.AWB_BaseUILayout_C|GetMenuStack (Variables|Default|GetBaseUIWidget))) PromptIndex))))

(event Custom|OnPromptCanceled_Event
  (params (PromptIndex :type UI_PromptIndex%20Enum :default "NewEnumerator0") (PromptToStack :type UI_PromptToStack%20Enum :default "NewEnumerator0"))
  ;[1 1 1] Exit Menu (Yes/ No)
  (switch Utilities|FlowControl|Switch|SwitchonUI_PromptToStack PromptToStack
    (:NewEnumerator0
      (Class|BPIPromptInterface|PromptCanceled(Message) (Class|CommonActivatableWidgetContainerBase|GetActiveWidget (Variables|/Game/Widgets/AWB/AWB_BaseUILayout.AWB_BaseUILayout_C|GetMenuStack (Variables|Default|GetBaseUIWidget))) (stale Custom|OnPromptConfirmed_Event PromptIndex)))))

(event Custom|Client_LeaveEIKLobby
  ;[1 1 1] Leave Session
  ;;[1 1 1] Each client individually leaves the EIK session
  (|DestroyEIKSessions (.ReturnValue (Class|EIKBlueprintFunctions|GetUserUniqueID self))
    (:OnSuccess
      (Game|OpenLevel(byObjectReference) "/Game/Maps/LobbyCreate.LobbyCreate"))))

(event Custom|Re-enablePlayMenu
  (bind _returnvalue (Class|EIKSubsystem|GetPlayerNickname))
  (bind _playmenuref (Variables|Default|GetPlayMenuRef))
  ;[1 1 1] Re-enable Play Menu
  (Widget|SetIsEnabled (Variables|Default|GetPlayMenuRef) true)
  (if (Utilities|Array|IsEmpty _returnvalue)
    (bind _playername (Class|BPIGameInstance|GetPlayerName(Message) (Game|GetGameInstance)))
    (Variables|/Script/UMG.EditableText|SetText (Variables|/Game/Widgets/AWB/AWB_Play.AWB_Play_C|GetName (Variables|Default|GetPlayMenuRef)) _playername)
    (else
      (Variables|/Script/UMG.EditableText|SetText (Variables|/Game/Widgets/AWB/AWB_Play.AWB_Play_C|GetName _playmenuref) (Utilities|Text|ToText(String) _returnvalue))
      (Widget|SetIsEnabled (Variables|/Game/Widgets/AWB/AWB_Play.AWB_Play_C|GetName _playmenuref) false))))

(event Custom|ServerSetPlayerNickname
  (params (PlayerNickname :type Text))
  (Class|BPIPlayerState|PSISetPlayerName(Message) (Variables|GetPlayerState) PlayerNickname))

(event Custom|ClientUpdatePlayerNickname
  (Class|BPILobbyBrowser|LBIUpdatePlayerNickname(Message) (Class|CommonActivatableWidgetContainerBase|GetActiveWidget (Variables|/Game/Widgets/AWB/AWB_BaseUILayout.AWB_BaseUILayout_C|GetMenuStack (Variables|Default|GetBaseUIWidget)))))

(event EventBeginPlay
  ;[1 1 1] Create BaseUI then base on level name create AWB
  (if (Pawn|IsLocalController)
    (Input|SetInputModeUIOnly self 0 "DoNotLock" false)
    (Variables|/Script/Engine.PlayerController|SetbShowMouseCursor self true)
    (bind _returnvalue (UserInterface|CreateWidget "/Game/Widgets/AWB/AWB_BaseUILayout.AWB_BaseUILayout_C" self))
    (bind _output_get (Variables|Default|SetBaseUIWidget _returnvalue))
    (UserInterface|Viewport|AddtoViewport _output_get 0)
    (bind _returnvalue_2 (Game|GetCurrentLevelName true))
    ;;[1 1 1] Push Menu base on level name
    (switch string _returnvalue_2
      (:MainMenu
        (bind _returnvalue_3 (Default|PushPlayMenu (Variables|Default|GetBaseUIWidget)))
        (Variables|Default|SetPlayMenuRef _returnvalue_3)
        (bind _returnvalue_4 (Actor|GetActorOfClass "/Game/Blueprints/BP_MasterBinderUI.BP_MasterBinderUI_C"))
        (Variables|Default|SetMasterBinderUI _returnvalue_4)
        (CallFunction|Bindings)
        (bind _islogin (Class|BPIGameInstance|GetIsLogin(Message) (Game|GetGameInstance)))
        (if (not _islogin)
          (Widget|SetIsEnabled (Variables|Default|GetPlayMenuRef) false)
          (Utilities|FlowControl|Delay 1.0)
          (bind _returnvalue_5 (Default|PushLoginMenu (Variables|Default|GetBaseUIWidget)))
          (bind _output_get_2 (Variables|Default|SetLoginMenuRef _returnvalue_5))
          (Variables|/Game/Widgets/AWB/AWB_Login.AWB_Login_C|SetMenuControllerRef _output_get_2 self)))
      (:LobbyCreate
        (Default|PushMenu (Variables|Default|GetBaseUIWidget) "/Game/Widgets/AWB/AWB_MainMenu.AWB_MainMenu_C"))
      (:Lobby
        (CameraFades|StartCameraFade :self (Game|GetPlayerCameraManager 0) :FromAlpha 5.0 :Duration 2.5)
        (Utilities|FlowControl|Delay 2.0)
        (bind _returnvalue_6 (Actor|GetActorOfClass "/Script/CinematicCamera.CineCameraActor"))
        (Game|Player|SetViewTargetwithBlend _returnvalue_6 0.0 "VTBlend_Linear" 0.0 false)
        (Default|PushMenu (Variables|Default|GetBaseUIWidget) "/Game/Widgets/AWB/AWB_Lobby.AWB_Lobby_C")
        (CallFunction|GetPlayerNickname)))))

(event EventPCWMPushMenuPrompt
  (params (PromptText :type Text) (PromptIndex :type UI_PromptIndex%20Enum :default "NewEnumerator0") (PromptToStack :type UI_PromptToStack%20Enum :default "NewEnumerator0"))
  ;[1 1 1] Menu Prompt With Custom Prompt (Quit)
  (Default|PushMenuPrompt (Variables|Default|GetBaseUIWidget) PromptIndex PromptToStack PromptText))

(event EventPCWMPushHUD
  (params (ActivatableWidget :type Common%20Activatable%20Widget%20Class%20Reference))
  (Default|PushHUD (Variables|Default|GetBaseUIWidget) ActivatableWidget))

(event EventPCWMPushMenu
  (params (ActivatableWidget :type Common%20Activatable%20Widget%20Class%20Reference))
  ;[1 1 1] Push Any AWB Menu
  (Default|PushMenu (Variables|Default|GetBaseUIWidget) ActivatableWidget))

(event EventPCILeaveEIKSession
  ;[1 1 1] Leave Session
  (CallFunction|ClientLeaveEIKLobby))

(event EventPCWMUpdatePlayerNickname
  (CallFunction|ClientUpdatePlayerNickname))

(fn ConstructionScript)

(fn GetPlayerNickname
  (bind _returnvalue (Class|EIKSubsystem|GetPlayerNickname))
  (bind _playername (Class|BPIGameInstance|GetPlayerName(Message) (Game|GetGameInstance)))
  (CallFunction|ServerSetPlayerNickname (select (Utilities|Array|IsEmpty _returnvalue) _playername (Utilities|Text|ToText(String) _returnvalue)))
  (return))

(fn PSIGetPlayerRole
  (return "NewEnumerator2"))

(fn PSIGetPlayerName
  (return ""))