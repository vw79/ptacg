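; BP_GraveGameState is a game state that runs the in-game clock on the Cemetery, Chinese and Tomb maps.
; On BeginPlay, the authority resets the replicated hour and minute and starts a looping timer that advances one game minute every few seconds.
; Each tick calls MulticastUpdateTime to refresh the time widget, which non-authority instances also call at start.
; At the hour limit the timer clears and only prints "Game Over".
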(event Custom|TimerStart
  ;[1 1 1] Calculate Time
  (if (Ability|HasAuthority)
    (Variables|Timer|SetRepCurrentHour 0)
    (Variables|Timer|SetRepCurrentMinute 0)
    (Utilities|Time|SetTimerbyFunctionName 0 "UpdateGameTime" 5.0 true)
    (else
      (CallFunction|MulticastUpdateTime))))

(event Custom|MulticastUpdateTime
  ;[1 1 1] Multicast Time Widget
  (Default|UpdateTime (Variables|Timer|GetWbpTimeRef) (Variables|Timer|GetRepCurrentHour) (Variables|Timer|GetRepCurrentMinute)))

(event EventBeginPlay
  (bind _returnvalue (Game|GetCurrentLevelName true))
  (switch string _returnvalue
    (:CementryMap
      _)
    (:ChineseMap
      _)
    (:TombMap
      _))
  (CallFunction|TimerStart))

(fn ConstructionScript)

(fn UpdateGameTime
  (bind _output_get (Variables|Timer|SetRepCurrentMinute (+ (Variables|Timer|GetRepCurrentMinute) 1)))
  (if (>= _output_get 60)
    (Variables|Timer|SetRepCurrentMinute 0)
    (bind _output_get_2 (Variables|Timer|SetRepCurrentHour (+ (Variables|Timer|GetRepCurrentHour) 1)))
    (if (>= _output_get_2 5)
      (Utilities|Time|ClearTimerbyFunctionName 0 "UpdateGameTime")
      (Development|PrintString "Game Over")))
  (CallFunction|MulticastUpdateTime))