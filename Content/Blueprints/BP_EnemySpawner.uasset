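; Enemy spawner actor that, on the server, uses a five-second looping timer to spawn a random Manny or Quinn character near a random reachable navmesh point around itself.
; Each spawn increments EnemyCount, but the logic that caps spawning and maps the count to effect weights is disconnected.
; BeginPlay creates vignette and chromatic aberration dynamic materials, which MulticastVignetteUpdate would blend into the post-process volume, though its only call here is unwired.
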(event Custom|Multicast%20Vignette%20Update
  (bind _ppvolumeref (Variables|PostProcess|GetPPVolumeRef))
  (bind _chromabweight (Variables|PostProcess|GetChromAbWeight))
  (bind _vignetteweight (Variables|PostProcess|GetVignetteWeight))
  ;[1 1 1] Multicast Vignette and ChromAb
  (Rendering|AddorUpdateBlendable _ppvolumeref (Variables|PostProcess|GetVigDynamicMat) _vignetteweight :!class /Script/Engine.PostProcessVolume)
  (Rendering|AddorUpdateBlendable _ppvolumeref (Variables|PostProcess|GetChromDynamicMat) _chromabweight :!class /Script/Engine.PostProcessVolume)
  (Development|PrintString (Utilities|String|Append (Utilities|String|ToString(Float) _vignetteweight) " " " " (Utilities|String|ToString(Float) _chromabweight))))

(event EventBeginPlay
  (bind _returnvalue (Actor|GetActorOfClass "/Script/Engine.PostProcessVolume"))
  (Variables|PostProcess|SetPPVolumeRef _returnvalue)
  (bind _returnvalue_2 (Rendering|Material|CreateDynamicMaterialInstance "/Game/PostProcessEffect/MI_Vignette_Inst.MI_Vignette_Inst" "None" "None" :!class /Script/Engine.KismetMaterialLibrary))
  (Variables|PostProcess|SetVigDynamicMat _returnvalue_2)
  (bind _returnvalue_3 (Rendering|Material|CreateDynamicMaterialInstance "/Game/PostProcessEffect/MI_ChromAb_Inst.MI_ChromAb_Inst" "None" "None" :!class /Script/Engine.KismetMaterialLibrary))
  (Variables|PostProcess|SetChromDynamicMat _returnvalue_3)
  ;[1 1 1] Only Spawn on Server
  (if (Ability|HasAuthority)
    (Utilities|Time|SetTimerbyFunctionName 0 "SpawnEnemy" 5.0 true)))

(fn ConstructionScript)

(fn SpawnEnemy
  (bind _returnvalue (Transformation|GetActorLocation))
  (bind _returnvalue_2 (Transformation|GetActorLocation))
  (bind _randomlocation (AI|Navigation|GetRandomReachablePointinRadius _returnvalue 5e+03 0 0))
  (bind _randomlocation_2 (AI|Navigation|GetRandomReachablePointinRadius _returnvalue_2 5e+03 0 0))
  (switch int (Math|Random|RandomIntegerinRange 0 1)
    (:0
      (Game|SpawnActorfromClass "/Game/Characters/BP_MannyCharacter.BP_MannyCharacter_C" (Math|Transform|MakeTransform (.location (Math|Transform|MakeTransform (Math|Vector|MakeVector (.x _randomlocation) (.y _randomlocation) (+ (.z _randomlocation) 1e+02)))) "0.000000,130.000000,0.000000" "1.000000,1.000000,1.000000") "AdjustIfPossibleButAlwaysSpawn" "MultiplyWithRoot" 0 0)
      (Math|Integer|IncrementInt (Variables|Spawn|GetEnemyCount)))
    (:1
      (Game|SpawnActorfromClass "/Game/Characters/BP_QuinnCharacter.BP_QuinnCharacter_C" (Math|Transform|MakeTransform (.location (Math|Transform|MakeTransform (Math|Vector|MakeVector (.x _randomlocation_2) (.y _randomlocation_2) (+ (.z _randomlocation_2) 1e+02)))) "0.000000,130.000000,0.000000" "1.000000,1.000000,1.000000") "Undefined" "MultiplyWithRoot" 0 0)
      (Math|Integer|IncrementInt (Variables|Spawn|GetEnemyCount)))))