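; Rotation puzzle Blueprint that turns a mesh in yaw steps and checks it against a target code linked to a door.
; A box overlap calls Rotate to turn right by RotateValue, though that call sets no target component.
; CheckCode tests yaw within a tolerance for only one mesh, StaticMeshComponent, updating CodeisGood.
; Both the pass and fail results call the door's SwitchOnOff, so it toggles either way.
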(event OnComponentBeginOverlap(Box)
  (params (OverlappedComponent :type Primitive%20Component%20Object%20Reference) (OtherActor :type Actor%20Object%20Reference) (OtherComp :type Primitive%20Component%20Object%20Reference) (OtherBodyIndex :type Integer) (bFromSweep :type Boolean) (SweepResult :type Hit%20Result%20Structure%20%28by%20ref%29))
  (CallFunction|Rotate 0 false))

(event OnComponentEndOverlap(Box)
  (params (OverlappedComponent :type Primitive%20Component%20Object%20Reference) (OtherActor :type Actor%20Object%20Reference) (OtherComp :type Primitive%20Component%20Object%20Reference) (OtherBodyIndex :type Integer)))

(fn ConstructionScript)

(fn Rotate
  (params (Component :type Primitive%20Component%20Object%20Reference) (RotateLeft :type Boolean))
  (if RotateLeft
    (Transformation|AddRelativeRotation Component (Math|Rotator|MakeRotator 0.0 0.0 (* (Variables|Default|GetRotateValue) -1.0)) false false)
    (else
      (Transformation|AddRelativeRotation Component (Math|Rotator|MakeRotator 0.0 0.0 (Variables|Default|GetRotateValue)) false false)))
  (CallFunction|CheckCode Component))

(fn CheckCode
  (params (Component :type Primitive%20Component%20Object%20Reference))
  (bind _door (Variables|Default|GetDoor))
  (if (== Component (Variables|Debug|GetStaticMeshComponent))
    (LocalVariables|SetSelectedMesh 0)
    (Utilities|Array|SetArrayElem (Variables|Default|GetCodeisGood) (LocalVariables|GetSelectedMesh) (Math|Float|NearlyEqual(Float) (Utilities|Array|Get(acopy) (Variables|Default|GetCode) (LocalVariables|GetSelectedMesh)) (.yaw (Variables|/Script/Engine.SceneComponent|GetRelativeRotation Component)) 1.0))
    (bind _array_element (Utilities|Array|ForEachLoopwithBreak (Variables|Default|GetCodeisGood) :!label _label)
      (:LoopBody
        (if (not _array_element)
          (LocalVariables|SetLocalFailed true)
          (goto _label Break)))
      (:Completed
        (if (LocalVariables|GetLocalFailed)
          (Default|SwitchOn/Off _door)
          (else
            (Default|SwitchOn/Off _door)))))))