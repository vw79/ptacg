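; BP_RotatePuzzleMaster is a rotating cylinder puzzle piece that switches a door when all pieces are finalized.
; RotateCylinder plays a timeline that turns the cylinder in 30-degree steps, ignores calls mid-move and tracks twelve wrapping positions.
; Each instance polls every cylinder's Finalize flag on a looping timer, then stops and toggles DoorRef.
; The answer comparison that sets Finalize is disconnected, so this graph never sets it.
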(event Custom|RotateCylinder
  (if (not (Variables|Default|GetCylinderMoving))
    (Variables|Default|SetCylinderMoving true)
    (bind _rotation (Timeline|RotateTime PlayFromStart)
      (:Update
        (Transformation|SetRelativeRotation (Variables|Default|GetCylinder) (Math|Rotator|MakeRotator (Math|Float|Lerp (.pitch (Variables|Default|GetStartingRotaion)) (- (.pitch (Variables|Default|GetStartingRotaion)) 3e+01) _rotation) 0.0 0.0) false false))
      (:Finished
        (Variables|Default|SetStartingRotaion (Math|Rotator|MakeRotator (Math|Float|Lerp (.pitch (Variables|Default|GetStartingRotaion)) (- (.pitch (Variables|Default|GetStartingRotaion)) 3e+01) _rotation) 0.0 0.0))
        (Variables|Default|SetCylinderMoving false)
        (bind _result (Math|Integer|IncrementInt (Variables|Default|GetCylinderPostition))
          (:%20%20
            (bind _output_get (Variables|Default|SetCylinderPostition _result))
            (if (> _output_get 11)
              (Variables|Default|SetCylinderPostition 0))))))))

(event Custom|PuzzleCheck
  (Variables|Default|SetPuzzleSolved true)
  (for _array_element (Variables|Default|GetAllCylinder)
    (if (not (Variables|BP_RotatePuzzleMaster_C|GetFinalize _array_element))
      (Variables|Default|SetPuzzleSolved false)))
  (if (Variables|Default|GetPuzzleSolved)
    (Utilities|Time|ClearandInvalidateTimerbyHandle (stale EventBeginPlay _returnvalue))
    (Default|SwitchOn/Off (Variables|Default|GetDoorRef))))

(event EventBeginPlay
  (Variables|Default|SetStartingRotaion (Variables|/Script/Engine.SceneComponent|GetRelativeRotation (Variables|Default|GetCylinder)))
  (bind _outactors (Actor|GetAllActorsOfClass "BP_RotatePuzzleMaster_C"))
  (Variables|Default|SetAllCylinder _outactors)
  (bind _returnvalue (Utilities|Time|SetTimerbyEvent (delegate Custom|PuzzleCheck) 0.25 true)))

(event EventTick
  (params (DeltaSeconds :type Float%20%28single-precision%29)))

(fn ConstructionScript)