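; Rotating cylinder puzzle piece that counts as solved when turned to its answer position among twelve steps.
; SwitchInteract sets Finalize by comparing the next position to PuzzleAnswer, then a timeline rolls the cylinder 30 degrees, ignoring rotation requests mid-turn.
; Each instance polls all cylinders on a looping timer, stopping and calling the puzzle-completed event once all are finalized.
; Tick prints position and solved state for debugging.
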(event Custom|RotateCylinder
  (if (not (Variables|Default|GetCylinderMoving))
    (Variables|Default|SetCylinderMoving true)
    (bind _rotation (Timeline|Rotation PlayFromStart)
      (:Update
        (Transformation|SetRelativeRotation (Variables|Default|GetCylinder) (Math|Rotator|MakeRotator (Math|Float|Lerp (.roll (Variables|Default|GetStartingRotation)) (- (.roll (Variables|Default|GetStartingRotation)) 3e+01) _rotation) 0.0 0.0) false false))
      (:Finished
        (Variables|Default|SetStartingRotation (Math|Rotator|MakeRotator (Math|Float|Lerp (.roll (Variables|Default|GetStartingRotation)) (- (.roll (Variables|Default|GetStartingRotation)) 3e+01) _rotation) 0.0 0.0))
        (Variables|Default|SetCylinderMoving false)
        (bind _result (Math|Integer|IncrementInt (Variables|Default|GetFramePosition))
          (:%20%20
            (bind _output_get (Variables|Default|SetFramePosition _result))
            (if (> _output_get 11)
              (Variables|Default|SetFramePosition 0))))))))

(event Custom|Puzzle%20Check
  (Variables|Default|SetPuzzleSolved true)
  (for _array_element (Variables|Default|GetAll%20Cylinder)
    (if (not (Variables|BP_RotatePuzzleM_C|GetFinalize _array_element))
      (Variables|Default|SetPuzzleSolved false)))
  (if (Variables|Default|GetPuzzleSolved)
    (Utilities|Time|ClearandInvalidateTimerbyHandle (stale EventBeginPlay _returnvalue))
    (Default|CallEVDPuzzleCompleted)))

(event EventBeginPlay
  (Variables|Default|SetStartingRotation (Variables|/Script/Engine.SceneComponent|GetRelativeRotation (Variables|Default|GetCylinder)))
  (bind _outactors (Actor|GetAllActorsOfClass "BP_RotatePuzzleM_C"))
  (Variables|Default|SetAll%20Cylinder _outactors)
  (bind _returnvalue (Utilities|Time|SetTimerbyEvent (delegate Custom|Puzzle%20Check) 0.25 true)))

(event EventTick
  (params (DeltaSeconds :type Float%20%28single-precision%29))
  (Development|PrintString (Utilities|String|ToString(Integer) (Variables|Default|GetFramePosition)) true true "(R=0.000000,G=0.660000,B=1.000000,A=1.000000)" DeltaSeconds)
  (Development|PrintString (Utilities|String|ToString(Boolean) (Variables|Default|GetFinalize)) true true "(R=0.000000,G=0.660000,B=1.000000,A=1.000000)" DeltaSeconds))

(event EventSwitchInteract
  (if (== (+ (Variables|Default|GetFramePosition) 1) (Variables|Default|GetPuzzleAnswer))
    (Variables|Default|SetFinalize true)
    (CallFunction|RotateCylinder)
    (else
      (Variables|Default|SetFinalize false)
      (CallFunction|RotateCylinder))))

(fn ConstructionScript
  (|CallParentFunction))