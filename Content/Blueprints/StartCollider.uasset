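; StartCollider is a trigger box that signals game start once both the Digger and the Attacker have left it.
; Its end-overlap event checks actor tags and latches an exited flag for each role.
; Both flags are tested only when an Attacker exits, so the Digger must already be out for the GameState's start message to be set.
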(event OnComponentEndOverlap(Box)
  (params (OverlappedComponent :type Primitive%20Component%20Object%20Reference) (OtherActor :type Actor%20Object%20Reference) (OtherComp :type Primitive%20Component%20Object%20Reference) (OtherBodyIndex :type Integer))
  (if (Actor|ActorHasTag OtherActor "Digger")
    (Variables|Default|SetDiggerExited true))
  (if (Actor|ActorHasTag OtherActor "Attacker")
    (Variables|Default|SetAttackerExited true)
    (if (and (Variables|Default|GetDiggerExited) (Variables|Default|GetAttackerExited))
      (Class|BPIGraveGameState|SetGameStart(Message) (Game|GetGameState) true))))

(fn ConstructionScript)