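; Coffin actor that lets the Digger player start a dig quick-time event when near it.
; Box overlap checks the Digger tag, facing via a dot product, and player-state role, then shows the press-F prompt and binds the HUD dig widget to this coffin's progress.
; Leaving the box hides both widgets.
; Open and disable events call multicasts that make the mesh ignore Visibility traces and turn off box collision.
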(event OnComponentEndOverlap(Box)
  (params (OverlappedComponent :type Primitive%20Component%20Object%20Reference) (OtherActor :type Actor%20Object%20Reference) (OtherComp :type Primitive%20Component%20Object%20Reference) (OtherBodyIndex :type Integer))
  (bind _bpdiggercharacter (Variables|Default|GetBpDiggerCharacter))
  (bind _hudref (Class|BPIPCWidgetManager|PCWMGetHUDRef(Message) (Pawn|GetController _bpdiggercharacter)))
  (Variables|/Game/Characters/BP_DiggerCharacter.BP_DiggerCharacter_C|SetisInCollider _bpdiggercharacter false)
  (Widget|SetVisibility (Variables|/Game/Widgets/AWB/AWB_DiggerMain.AWB_DiggerMain_C|GetPressF _hudref) "Hidden")
  (Variables|/Game/Characters/BP_DiggerCharacter.BP_DiggerCharacter_C|SetisVisible _bpdiggercharacter false))

(event OnComponentBeginOverlap(Box)
  (params (OverlappedComponent :type Primitive%20Component%20Object%20Reference) (OtherActor :type Actor%20Object%20Reference) (OtherComp :type Primitive%20Component%20Object%20Reference) (OtherBodyIndex :type Integer) (bFromSweep :type Boolean) (SweepResult :type Hit%20Result%20Structure%20%28by%20ref%29))
  (if (Actor|ActorHasTag OtherActor "Digger")
    (bind _returnvalue (CallFunction|IsFacing OtherActor OtherActor))
    (if _returnvalue
      (bind _playerrole (Class|BPIPlayerState|PSIGetPlayerRole(Message) (Game|GetPlayerState 0)))
      (switch Utilities|FlowControl|Switch|SwitchonPlayerRole _playerrole
        (:NewEnumerator0
          (bind _returnvalue_2 (Actor|GetActorOfClass "/Game/Characters/BP_DiggerCharacter.BP_DiggerCharacter_C"))
          (bind _hudref (Class|BPIPCWidgetManager|PCWMGetHUDRef(Message) (Pawn|GetController _returnvalue_2)))
          (Variables|/Game/Widgets/Modular/WBP_QTEDig.WBP_QTEDig_C|SetHitboxRef (Variables|/Game/Widgets/AWB/AWB_DiggerMain.AWB_DiggerMain_C|GetWBP_QTEDig _hudref) self)
          (Variables|Default|SetBpDiggerCharacter _returnvalue_2)
          (Default|ResetCount (Variables|/Game/Widgets/AWB/AWB_DiggerMain.AWB_DiggerMain_C|GetWBP_QTEDig _hudref) (Variables|Default|GetProgressCount))
          (Variables|/Game/Characters/BP_DiggerCharacter.BP_DiggerCharacter_C|SetisInCollider _returnvalue_2 true)
          (Widget|SetVisibility (Variables|/Game/Widgets/AWB/AWB_DiggerMain.AWB_DiggerMain_C|GetPressF _hudref) "Visible")
          (Variables|Default|SetWBP%20QTEDig (Variables|/Game/Widgets/AWB/AWB_DiggerMain.AWB_DiggerMain_C|GetWBP_QTEDig _hudref)))))
    (else
      (Development|PrintString "You are not digger"))))

(event Custom|MulticastOpenCoffin
  ;[1 1 1] Open Coffin
  (Collision|SetCollisionResponsetoChannel (Variables|Default|GetStaticMeshComponent1) "ECC_Visibility" "ECR_Ignore"))

(event Custom|MulticastDisableFBox
  ;[1 1 1] Disable F Box
  (Collision|SetCollisionEnabled (Variables|Default|GetBox) "NoCollision"))

(event EventOpenCoffin
  ;[1 1 1] Open Coffin
  (CallFunction|MulticastOpenCoffin))

(event EventDisableFBox
  ;[1 1 1] Disable F Box
  (CallFunction|MulticastDisableFBox))

(fn ConstructionScript)

(fn IsFacing
  (params (ActorForwardVector :type Actor%20Object%20Reference) (ActorLocation :type Actor%20Object%20Reference))
  (bind _output_get (Variables|Default|SetDirectionToCollider (- (Transformation|GetActorLocation) (Transformation|GetActorLocation ActorLocation))))
  (return (> (Math|Vector|DotProduct (Transformation|GetActorForwardVector ActorForwardVector) _output_get) 0.0)))